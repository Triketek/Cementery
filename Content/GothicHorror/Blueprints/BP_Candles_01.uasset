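; Candle prop with a point light and three particle systems, with a construction-time LightOn switch that shows or hides them.
; Tick eases the light toward a random horizontal offset around its starting position, re-picked after short random delays, to fake flickering flames.
; Toggle reads a scalar from the MPCTOD material parameter collection, hiding light and particles when it is above zero and showing them otherwise.
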(event `self.ReceiveTick`
  (params (DeltaSeconds :type "Float (single-precision)"))
  (bind _default_location (`self.Default Location`))
  (bind _pointlight (`self.PointLight`))
  (`SceneComponent.K2_SetWorldLocation` _pointlight (`KismetMathLibrary.VLerp` (`SceneComponent.K2_GetComponentLocation` _pointlight) (`self.New Location`) DeltaSeconds) false false)
  (`KismetSystemLibrary.Delay` (`KismetMathLibrary.RandomFloatInRange` 0.1 0.2))
  (set `self.New Location` (`KismetMathLibrary.MakeVector` (.x (+ (* (`KismetMathLibrary.RandomUnitVector`) 10.0) _default_location)) (.y (+ (* (`KismetMathLibrary.RandomUnitVector`) 10.0) _default_location)) (.z _default_location))))

(event `/Game/GothicHorror/Blueprints/BPI_Switchable.Toggle`
  (bind _pointlight (`self.PointLight`))
  (bind _returnvalue (`KismetMaterialLibrary.GetScalarParameterValue` (`self.MPCTOD`) (`self.Parameter Name`)))
  (if (> _returnvalue 0.0)
    (`SceneComponent.SetHiddenInGame` _pointlight true false)
    (`SceneComponent.SetHiddenInGame` (`self.ParticleSystem`) true false)
    (`SceneComponent.SetHiddenInGame` (`self.ParticleSystem1`) true false)
    (`SceneComponent.SetHiddenInGame` (`self.ParticleSystem2`) true false)
    (else
      (`SceneComponent.SetHiddenInGame` _pointlight false false)
      (`SceneComponent.SetHiddenInGame` (`self.ParticleSystem`) false false)
      (`SceneComponent.SetHiddenInGame` (`self.ParticleSystem1`) false false)
      (`SceneComponent.SetHiddenInGame` (`self.ParticleSystem2`) false false))))

(fn `UserConstructionScript`
  (bind _pointlight (`self.PointLight`))
  (bind _light_on (`self.Light On`))
  (bind _output_get (set `self.Default Location` (`SceneComponent.K2_GetComponentLocation` (`self.PointLight`))))
  (set `self.New Location` _output_get)
  (`SceneComponent.SetHiddenInGame` _pointlight (not _light_on) false)
  (`SceneComponent.SetHiddenInGame` (`self.ParticleSystem1`) (not _light_on) false)
  (`SceneComponent.SetHiddenInGame` (`self.ParticleSystem2`) (not _light_on) false)
  (`SceneComponent.SetHiddenInGame` (`self.ParticleSystem`) (not _light_on) false)
  (`SceneComponent.SetVisibility` _pointlight _light_on false)
  (`SceneComponent.SetVisibility` (`self.ParticleSystem1`) _light_on false)
  (`SceneComponent.SetVisibility` (`self.ParticleSystem2`) _light_on false)
  (`SceneComponent.SetVisibility` (`self.ParticleSystem`) _light_on false))